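; Side-scrolling skeleton enemy that switches to a faster chase speed when pawn sensing spots a pawn.
; Its state enum is pushed to a Blackboard for the AI, changing on sighting, damage and death.
; Damage triggers PaperZD-style animation node jumps, and death disables capsule collision before delayed destruction.
; Melee triggers damage knights overlapping the hit box, while Tick snaps yaw to face the X movement direction.
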(event OnSeePawn(PawnSensing)
  (params (Pawn :type Pawn%20Object%20Reference))
  (if (Utilities|Enum|Equal(Enum) (Variables|Default|GetEnemyState) "NewEnumerator0")
    (Variables|Default|SetEnemyState "NewEnumerator1")
    (CallFunction|UpdateAiState)
    (Variables|Default|SetRunPlayRate 1.5)
    (Variables|/Script/Engine.CharacterMovementComponent|SetMaxWalkSpeed (Variables|Character|GetCharacterMovement) 2.5e+02)))

(event Custom|MeleeAttack
  (Variables|Default|SetIsAttacking true))

(event Custom|UpdateAiState
  (AI|Components|Blackboard|SetValueasEnum (AI|GetBlackboard (AI|GetAIController self)) (Utilities|Name|MakeLiteralName "State") (Variables|Default|GetEnemyState)))

(event EventBeginPlay
  (Variables|Default|SetEnemyState "NewEnumerator0")
  (CallFunction|UpdateAiState)
  (Variables|Default|SetRunPlayRate 1.0)
  (Variables|/Script/Engine.CharacterMovementComponent|SetMaxWalkSpeed (Variables|Character|GetCharacterMovement) 1.5e+02))

(event EventMeleeTrigger
  (CallFunction|HitCheck))

(event EventTick
  (params (DeltaSeconds :type Float%20%28single-precision%29))
  (bind _returnvalue (Transformation|GetActorRotation))
  (if (or (!= (.yaw _returnvalue) 0.0) (!= (.yaw _returnvalue) 1.8e+02))
    (Math|Float|CompareFloat (.x (Transformation|GetVelocity)) 0.0
      (:>
        (Transformation|SetActorRotation "0, 0, 0"))
      (:<
        (Transformation|SetActorRotation "0.000000,180.000000,0.000000")))))

(event Game|Damage|EventAnyDamage
  (params (Damage :type Float%20%28single-precision%29) (DamageType :type Damage%20Type%20Object%20Reference) (InstigatedBy :type Controller%20Object%20Reference) (DamageCauser :type Actor%20Object%20Reference))
  (if (not (Variables|Default|GetIsDead))
    (bind _output_get (Variables|Default|SetHealth (- (Variables|Default|GetHealth) Damage)))
    (if (<= _output_get 0.0)
      (Class|PaperZDAnimInstance|JumptoNode (Variables|/Script/PaperZD.PaperZDAnimationComponent|GetAnimInstance (Variables|Default|GetAnimationComponent)) "Dead" "None")
      (Variables|Default|SetIsDead true)
      (Collision|SetCollisionEnabled (Variables|Default|GetCapsuleComponent) "NoCollision")
      (Variables|Default|SetEnemyState "NewEnumerator3")
      (CallFunction|UpdateAiState)
      (Utilities|FlowControl|Delay 1e+01)
      (Actor|DestroyActor)
      (else
        (Class|PaperZDAnimInstance|JumptoNode (Variables|/Script/PaperZD.PaperZDAnimationComponent|GetAnimInstance (Variables|Default|GetAnimationComponent)) "Damage" "None")
        (Components|Movement|StopMovementImmediately (Variables|Character|GetCharacterMovement))
        (Variables|Default|SetEnemyState "NewEnumerator2")
        (CallFunction|UpdateAiState)))))

(fn ConstructionScript)

(fn HitCheck
  (for _array_element (Collision|GetOverlappingActors (Variables|Default|GetHit%20Box) "/Game/Resource/Blueprints/Player/BP_Knight.BP_Knight_C" :!class /Script/Engine.PrimitiveComponent)
    (if (!= _array_element self)
      (Game|Damage|ApplyDamage _array_element 1.0 0 0))))